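; Stadium player pawn with a Paper2D sprite that performs a single hit on input while CanHit is true.
; On BeginPlay it gets possessed, adds the IMC_Stadium input context and switches the view to a level camera.
; A double-speed timeline slides the sprite to HitEndLocation, swaps in the hit sprite and sets the GM_Stadium phase.
; Reset restores the idle sprite and default position and leaves hitting disabled.
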(event Custom|PerformHit
  (Components|Timeline|SetPlayRate (Variables|Default|GetPerformHitTL) 2.0)
  (bind _alpha (Timeline|PerformHitTL PlayFromStart)
    (:Update
      (CallFunction|LerpSpritePos (Variables|Default|GetDefaultSpritePos) (Variables|/Script/Engine.SceneComponent|GetRelativeLocation (Variables|Default|GetHitEndLocation)) _alpha))
    (:ChangeSprite
      (CallFunction|ChangeSpriteto (Variables|Default|GetHitSprite))))
  (bind _asgm_stadium (Utilities|Casting|CastToGM_Stadium (Game|GetGameMode)))
  (Variables|/Game/Dynamic/Blueprints/GM_Stadium.GM_Stadium_C|SetPhase _asgm_stadium "NewEnumerator2"))

(event Input|EnhancedActionEvents|EnhancedInputActionIA_Hit
  (params (ActionValue :type Boolean) (ElapsedSeconds :type Float%20%28double-precision%29) (TriggeredSeconds :type Float%20%28double-precision%29) (InputAction :type Input%20Action%20Object%20Reference :default "/Game/Dynamic/Input/Actions/IA_Hit.IA_Hit"))
  (:Started
    (if (Variables|Default|GetCanHit)
      (CallFunction|PerformHit)
      (Variables|Default|SetCanHit false))))

(event EventBeginPlay
  (Pawn|Possess (Game|GetPlayerController 0) self)
  (bind _asplayer_controller (Utilities|Casting|CastToPlayerController (Pawn|GetController)))
  (Input|AddMappingContext (PlayerController|LocalPlayerSubsystems|GetEnhancedInputLocalPlayerSubsystem _asplayer_controller) "/Game/Dynamic/Input/IMC_Stadium.IMC_Stadium" 0 "(bIgnoreAllPressedKeysUntilRelease=True,bForceImmediately=False)")
  (bind _returnvalue (Actor|GetActorOfClass "/Script/Engine.CameraActor"))
  (Game|Player|SetViewTargetwithBlend (Game|GetPlayerController 0) _returnvalue 0.0 "VTBlend_Linear" 0.0 false)
  (CallFunction|ChangeSpriteto (Variables|Default|GetIdleSprite)))

(event Collision|EventActorBeginOverlap
  (params (OtherActor :type Actor%20Object%20Reference)))

(event EventTick
  (params (DeltaSeconds :type Float%20%28single-precision%29)))

(fn ConstructionScript)

(fn ChangeSpriteto
  (params (NewSprite :type Paper%20Sprite%20Object%20Reference))
  (Rendering|Components|Sprite|SetSprite (Variables|Default|GetPaperSprite) NewSprite)
  (Rendering|Material|SetMaterial (Variables|Default|GetPaperSprite) 0 "/Paper2D/TranslucentUnlitSpriteMaterial.TranslucentUnlitSpriteMaterial")
  (Rendering|SetTranslucentSortPriority (Variables|Default|GetPaperSprite) 2)
  (Rendering|SetVisibility (Variables|Default|GetPaperSprite) true false))

(fn LerpSpritePos
  (params (A :type Vector) (B :type Vector) (Alpha :type Float%20%28single-precision%29))
  (Transformation|SetRelativeLocation (Variables|Default|GetPaperSprite) (Math|Vector|Lerp(Vector) A B Alpha) false false))

(fn Reset
  (Variables|Default|SetCanHit false)
  (CallFunction|ChangeSpriteto (Variables|Default|GetIdleSprite))
  (Transformation|SetRelativeLocation (Variables|Default|GetPaperSprite) (Variables|Default|GetDefaultSpritePos) false false))